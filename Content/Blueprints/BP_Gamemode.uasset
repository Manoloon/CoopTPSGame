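; Game mode Blueprint that spawns BP_trackerball bots on demand through its SpawnNewBot event.
; SpawnNewBot runs the EQS_FindBotSpawn query in random-best-25% mode and, on success, spawns a bot at each returned location, adjusting for collisions.
; The random class pick has BP_trackerball on both branches, so it has no effect.
; BeginPlay is empty, and a delayed NetworkManager spawn is left unconnected.
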(event `self.SpawnNewBot`
  (bind _returnvalue (`EnvQueryManager.RunEQSQuery` "/Game/Blueprints/EQS_FindBotSpawn.EQS_FindBotSpawn" self "RandomBest25Pct"))
  (add `EnvQueryInstanceBlueprintWrapper.OnQueryFinishedEvent` _returnvalue (delegate `OnQueryFinishedEvent_Event_0`)))

(event `OnQueryFinishedEvent_Event_0`
  (params (QueryInstance :type "EnvQueryInstanceBlueprintWrapper Object Reference") (QueryStatus :type "EEnvQueryStatus Enum" :default "Processing"))
  (switch `EEnvQueryStatus` QueryStatus
    (:`Success`
      (bind (_resultlocations _returnvalue) (`EnvQueryInstanceBlueprintWrapper.GetQueryResultsAsLocations` QueryInstance))
      (if _returnvalue
        (for _array_element _resultlocations
          (`|SpawnActorFromClass` (select `bool` (>= (`KismetMathLibrary.RandomFloatInRange` 0.0 100.0) 35.0) :`false` "/Game/Blueprints/BP_trackerball.BP_trackerball_C" :`true` "/Game/Blueprints/BP_trackerball.BP_trackerball_C" :!type "Actor Class Reference") (`KismetMathLibrary.MakeTransform` _array_element) "AdjustIfPossibleButAlwaysSpawn" "OverrideRootScale" null null))))))

(event `self.ReceiveBeginPlay`)

(fn `UserConstructionScript`)