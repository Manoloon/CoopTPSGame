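; Test game mode that spawns AI bots and holds logic for awarding kill score.
; SpawnNewBot runs an EQS query and spawns a randomly chosen advanced AI or, less often, tracker ball at each returned location.
; A kill handler adds score to the killer's player state when the victim is not locally controlled, but its delegate binding is never executed here.
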(event `self.SpawnNewBot`
  (bind _returnvalue (`EnvQueryManager.RunEQSQuery` "/Game/Blueprints/EQS_FindBotSpawn.EQS_FindBotSpawn" self "RandomBest25Pct"))
  (add `EnvQueryInstanceBlueprintWrapper.OnQueryFinishedEvent` _returnvalue (delegate `OnQueryFinishedEvent_Event_0`)))

(event `OnQueryFinishedEvent_Event_0`
  (params (QueryInstance :type "EnvQueryInstanceBlueprintWrapper Object Reference") (QueryStatus :type "EEnvQueryStatus Enum" :default "Processing"))
  (switch `EEnvQueryStatus` QueryStatus
    (:`Success`
      (bind _resultlocations (`EnvQueryInstanceBlueprintWrapper.GetQueryResultsAsLocations` QueryInstance))
      (for _array_element _resultlocations
        (`|SpawnActorFromClass` (select `bool` (>= (`KismetMathLibrary.RandomFloatInRange` 0.0 100.0) 35.0) :`false` "/Game/Blueprints/BP_trackerball.BP_trackerball_C" :`true` "/Game/AdvancedAI/BP_AdvancedAI.BP_AdvancedAI_C" :!type "Actor Class Reference") (`KismetMathLibrary.MakeTransform` _array_element) "AdjustIfPossibleButAlwaysSpawn" "OverrideRootScale" null null)))))

(event `self.ReceiveBeginPlay`)

(event `OnActorKilled_Event_0` :!signature `self.OnActorKilled`
  (params (VictimActor :type "Actor Object Reference") (KillerActor :type "Actor Object Reference") (KillerController :type "Controller Object Reference"))
  ;[1 1 1] no reward if kill a friend
  (bind _aspawn (cast `Pawn` VictimActor))
  (if (not (`Pawn.IsLocallyControlled` _aspawn))
    (bind _assplayer_state (cast `SPlayerState` (`Pawn.PlayerState` (`Controller.K2_GetPawn` KillerController)))
      (:`then`
        (`SPlayerState.AddScore` _assplayer_state 20.0))
      (:`CastFailed`
        (`KismetSystemLibrary.PrintString` "CAST FAILS!!!" true true (struct :`G` 0.66 :`B` 1.0 :`A` 1.0) 20.0)))))

(fn `UserConstructionScript`)