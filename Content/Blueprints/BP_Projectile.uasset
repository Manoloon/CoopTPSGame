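; BP_Projectile is a timed explosive actor that detonates one second after BeginPlay, regardless of impact.
; BeginPlay waits, spawns an explosion emitter and draws a debug sphere showing the damage radius.
; It then applies full radial damage without falloff, attributed to itself and its instigator controller, and destroys itself.
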(event `self.ReceiveBeginPlay`
  (bind _returnvalue (`self.K2_GetActorLocation`))
  (`KismetSystemLibrary.Delay` 1.0)
  (`GameplayStatics.SpawnEmitterAtLocation` "/Game/Effects/WeaponEffects/Explosion/P_Explosion.P_Explosion" (`self.K2_GetActorLocation`))
  (`KismetSystemLibrary.DrawDebugSphere` _returnvalue (`self.damageRadius`) 12 (struct :`R` 1.0 :`B` 0.068094 :`A` 1.0) 1.0 3.0)
  (`GameplayStatics.ApplyRadialDamage` :`BaseDamage` 20.0 :`Origin` _returnvalue :`DamageRadius` (`self.damageRadius`) :`DamageTypeClass` "/Script/Engine.DamageType" :`DamageCauser` self :`InstigatedByController` (`self.GetInstigatorController`) :`bDoFullDamage` true)
  (`self.K2_DestroyActor`))

(fn `UserConstructionScript`)