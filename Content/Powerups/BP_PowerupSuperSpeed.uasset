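; BP_PowerupSuperSpeed is a powerup that temporarily makes the first player's pawn walk ten times faster.
; On activation it calls the parent logic, then, if a CharacterMovementComponent exists, sets MaxWalkSpeed to ten times GetMaxSpeed.
; On expiry it divides GetMaxSpeed by the same factor instead of restoring a saved value, without a validity check, then calls the parent.
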(event `self.OnActivated`
  (bind _returnvalue (`self.GetComponentByClass` (`GameplayStatics.GetPlayerPawn` 0) "/Script/Engine.CharacterMovementComponent"))
  (`parent.OnActivated`)
  (`/Engine/EditorBlueprintResources/StandardMacros.IsValid` _returnvalue
    (:`Is Valid`
      (set `CharacterMovementComponent.MaxWalkSpeed` (* (`MovementComponent.GetMaxSpeed` _returnvalue) 10.0) _returnvalue))))

(event `self.OnExpired`
  (bind _returnvalue (`self.GetComponentByClass` (`GameplayStatics.GetPlayerPawn` 0) "/Script/Engine.CharacterMovementComponent"))
  (set `CharacterMovementComponent.MaxWalkSpeed` (/ (`MovementComponent.GetMaxSpeed` _returnvalue) 10.0) _returnvalue)
  (`parent.OnExpired`))

(fn `UserConstructionScript`)